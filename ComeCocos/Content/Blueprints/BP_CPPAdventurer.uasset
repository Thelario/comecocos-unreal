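; BP_CPPAdventurer is a player pawn that moves in fixed steps on WASD key presses.
; On BeginPlay it has the first player controller possess it.
; Each key press instantly offsets its location along the world X or Y axis by a set distance, without sweeping, so collision does not block the moves.
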(event `self.ReceiveBeginPlay`
  (`Controller.Possess` (`GameplayStatics.GetPlayerController` 0) self))

(event `Key|A`
  (params (Key :type "Key Structure"))
  (:`Pressed`
    (`self.K2_SetActorLocation` (+ (`self.K2_GetActorLocation`) (0.0 -200.0 0.0)))))

(event `Key|D`
  (params (Key :type "Key Structure"))
  (:`Pressed`
    (`self.K2_SetActorLocation` (+ (`self.K2_GetActorLocation`) (0.0 200.0 0.0)))))

(event `Key|W`
  (params (Key :type "Key Structure"))
  (:`Pressed`
    (`self.K2_SetActorLocation` (+ (`self.K2_GetActorLocation`) (200.0 0.0 0.0)))))

(event `Key|S`
  (params (Key :type "Key Structure"))
  (:`Pressed`
    (`self.K2_SetActorLocation` (+ (`self.K2_GetActorLocation`) (-200.0 0.0 0.0)))))

(fn `UserConstructionScript`)